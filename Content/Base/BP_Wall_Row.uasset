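; BP_Wall_Row is a moving wall row that builds itself from bricks and pivots.
; SetUpRow loops over BrickNumber, adding evenly spaced child actor components along local Y, either BP_Brick_01 or a scaled-down, rotated BP_Pivot.
; A counter checked against PatternID advances and wraps an index bounded by PatternArray's length, which selects the piece type.
; Tick moves the whole row by RowSpeed scaled by delta time, without sweeping.
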(event `SetUpRow`
  (for _index (range (`self.BrickNumber`))
    (if (>= (`self.CurrentID`) (`self.PatternID`))
      (bind _output_get (set `self.ArrayID` (+ (`self.ArrayID`) 1)))
      (if (> _output_get (`KismetArrayLibrary.Array_Length` (`self.PatternArray`)))
        (set `self.ArrayID` 0)))
    (switch `int` (`self.ArrayID`)
      (:`0`
        (bind _returnvalue (`AddComponent|NODE_AddChildActorComponent-1` :`RelativeTransform` (`KismetMathLibrary.MakeTransform` (* (0.0 115.0 0.0) _index))))
        (`ChildActorComponent.SetChildActorClass` _returnvalue "/Game/Environment/BlueprintsEnvironment/BP_Brick_01.BP_Brick_01_C"))
      (:`1`
        (bind _returnvalue_2 (`AddComponent|NODE_AddChildActorComponent-2` :`RelativeTransform` (`KismetMathLibrary.MakeTransform` (* (0.0 115.0 0.0) _index) (struct :`Yaw` 90.0) (0.1 0.1 0.1))))
        (`ChildActorComponent.SetChildActorClass` _returnvalue_2 "/Game/Environment/BlueprintsEnvironment/BP_Pivot.BP_Pivot_C")))
    (set `self.CurrentID` (+ (`self.CurrentID`) 1))))

(event `self.ReceiveTick`
  (params (DeltaSeconds :type "Float (single-precision)"))
  (`self.K2_SetActorLocation` (+ (`self.K2_GetActorLocation`) (* (`self.RowSpeed`) (`GameplayStatics.GetWorldDeltaSeconds`)))))

(fn `UserConstructionScript`)