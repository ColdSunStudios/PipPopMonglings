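; Ping-pong ball actor driven by a ProjectileMovement component that changes speed according to the paddle it bounces off.
; Tick applies custom vertical acceleration from GravityScale and derives the ball's rotation from its velocity.
; On bounce off a BP_PlayerPaddle it prints a debug message, then speeds up if the paddle is Powered or slows down if Weakened.
; Overlap handling and look-at-based deflection experiments remain disconnected.
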(event `self.ReceiveTick`
  (params (DeltaSeconds :type "Float (single-precision)"))
  (bind _projectilemovement (`self.ProjectileMovement`))
  (bind _output_get (set `MovementComponent.Velocity` (+ (`MovementComponent.Velocity` _projectilemovement) (* (0.0 0.0 1.0) (* DeltaSeconds (`self.GravityScale`)))) _projectilemovement))
  (`self.K2_SetActorRotation` (`KismetMathLibrary.MakeRotationFromAxes` (0.0 0.0 0.0) (`KismetMathLibrary.GreaterGreater_VectorRotator` _output_get (struct :`Pitch` 1.0 :`Yaw` 1.0 :`Roll` 1.0)))))

(event `self.Sphere1.OnComponentBeginOverlap`
  (params (OverlappedComponent :type "PrimitiveComponent Object Reference") (OtherActor :type "Actor Object Reference") (OtherComp :type "PrimitiveComponent Object Reference") (OtherBodyIndex :type Integer) (bFromSweep :type Boolean) (SweepResult :type "HitResult Structure (by ref)")))

(event `self.Sphere1.OnComponentHit`
  (params (HitComponent :type "PrimitiveComponent Object Reference") (OtherActor :type "Actor Object Reference") (OtherComp :type "PrimitiveComponent Object Reference") (NormalImpulse :type "Vector Structure") (Hit :type "HitResult Structure (by ref)")))

(event `self.ProjectileMovement.OnProjectileBounce`
  (params (ImpactResult :type "HitResult Structure (by ref)") (ImpactVelocity :type "Vector Structure (by ref)"))
  (bind _projectilemovement (`self.ProjectileMovement`))
  (bind _projectilemovement_2 (`self.ProjectileMovement`))
  (bind _asbp_player_paddle (cast `/Game/Player/BP_PlayerPaddle` (`.HitActor` (`GameplayStatics.BreakHitResult` ImpactResult))))
  (`KismetSystemLibrary.PrintString` "Paddle hit!" true true (struct :`G` 1.0 :`B` 0.215381 :`A` 1.0))
  (if (`/Game/Player/BP_PlayerPaddle.Powered` _asbp_player_paddle)
    (set `MovementComponent.Velocity` (* (`MovementComponent.Velocity` _projectilemovement) 1.5) _projectilemovement)
    (elif (`/Game/Player/BP_PlayerPaddle.Weakened` _asbp_player_paddle)
      (set `MovementComponent.Velocity` (/ (`MovementComponent.Velocity` _projectilemovement_2) 1.5) _projectilemovement_2))))

(fn `UserConstructionScript`)