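; BP_Wall_Master is a brick wall builder that assembles a wall from stacked BP_Wall_Row actors.
; The construction script adds one child actor component per row, spacing them vertically at a fixed interval up to RowNumber.
; Each row gets either the shared BricksPerRow count or a random count between MinBricks and MaxBricks, then runs SetUpRow.
; The event graph holds no active logic.
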(fn `UserConstructionScript`
  (for _index (range (`self.RowNumber`))
    (bind _returnvalue (`AddComponent|NODE_AddChildActorComponent-0` :`RelativeTransform` (`KismetMathLibrary.MakeTransform` (* (0.0 0.0 50.0) _index))))
    (`ChildActorComponent.SetChildActorClass` _returnvalue "/Game/Base/BP_Wall_Row.BP_Wall_Row_C")
    (if (`self.RandomiseBrickNumber`)
      (bind _asbp_wall_row (cast `/Game/Base/BP_Wall_Row` (`ChildActorComponent.ChildActor` _returnvalue) :!pure true))
      (set `/Game/Base/BP_Wall_Row.BrickNumber` (`KismetMathLibrary.RandomIntegerInRange` (`self.MinBricks`) (`self.MaxBricks`)) _asbp_wall_row)
      (else
        (set `/Game/Base/BP_Wall_Row.BrickNumber` (`self.BricksPerRow`) _asbp_wall_row)))
    (`/Game/Base/BP_Wall_Row.SetUpRow` _asbp_wall_row)))