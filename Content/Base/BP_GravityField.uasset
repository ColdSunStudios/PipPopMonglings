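; BP_GravityField is a gravity field actor that inverts the gravity of ping pong balls entering its wells.
; On BeginPlay it snaps its world X position to zero, keeping Y and Z.
; Begin overlap on either GravityWell_Top or GravityWell_Bottom casts the other actor to BP_PingPongBall and negates its GravityScale.
; Each overlap flips the current value, so successive entries alternate the gravity direction.
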(event `self.ReceiveBeginPlay`
  (`self.K2_SetActorLocation` (`KismetMathLibrary.MakeVector` 0.0 (.y (`self.K2_GetActorLocation`)) (.z (`self.K2_GetActorLocation`)))))

(event `self.GravityWell_Bottom.OnComponentBeginOverlap`
  (params (OverlappedComponent :type "PrimitiveComponent Object Reference") (OtherActor :type "Actor Object Reference") (OtherComp :type "PrimitiveComponent Object Reference") (OtherBodyIndex :type Integer) (bFromSweep :type Boolean) (SweepResult :type "HitResult Structure (by ref)"))
  (bind _asbp_ping_pong_ball (cast `/Game/Base/BP_PingPongBall` OtherActor))
  (bind _output_get (set `/Game/Base/BP_PingPongBall.GravityScale` (* (`/Game/Base/BP_PingPongBall.GravityScale` _asbp_ping_pong_ball) -1.0) _asbp_ping_pong_ball)))

(event `self.GravityWell_Top.OnComponentBeginOverlap`
  (params (OverlappedComponent :type "PrimitiveComponent Object Reference") (OtherActor :type "Actor Object Reference") (OtherComp :type "PrimitiveComponent Object Reference") (OtherBodyIndex :type Integer) (bFromSweep :type Boolean) (SweepResult :type "HitResult Structure (by ref)"))
  (bind _asbp_ping_pong_ball (cast `/Game/Base/BP_PingPongBall` OtherActor))
  (bind _output_get (set `/Game/Base/BP_PingPongBall.GravityScale` (* (`/Game/Base/BP_PingPongBall.GravityScale` _asbp_ping_pong_ball) -1.0) _asbp_ping_pong_ball)))

(fn `UserConstructionScript`)