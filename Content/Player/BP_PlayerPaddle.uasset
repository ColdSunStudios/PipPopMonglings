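; Ping-pong paddle pawn, playable by the player or a bot via IsBot.
; The player version spawns the ball, switches to the ortho camera, moves by axis input and rotates toward the cursor deprojected onto X=0.
; The bot takes an AIController, lerps under the ball in a zero-delay loop and randomly toggles power states on hits.
; Mouse-button Powered and Weakened timelines resize mesh, collider and sprite, updating the bot's clamp bounds.
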(event `MoveUnderBall`
  (bind _returnvalue (`self.K2_GetActorLocation`))
  (bind _outactors (`GameplayStatics.GetAllActorsOfClass` "/Game/Base/BP_PingPongBall.BP_PingPongBall_C"))
  (for _array_element _outactors
    (set `self.BallReference` _array_element))
  (`self.K2_SetActorLocation` self (`KismetMathLibrary.VLerp` _returnvalue (`KismetMathLibrary.MakeVector` (.x _returnvalue) (`KismetMathLibrary.FClamp` (.y (`self.K2_GetActorLocation` (`self.BallReference`))) -310.0 310.0) (.z _returnvalue)) (* (`GameplayStatics.GetWorldDeltaSeconds`) (`self.BotMoveSpeed`))) false false)
  (`KismetSystemLibrary.Delay` 0.0)
  (`self.MoveUnderBall`))

(event `SetUpBot`
  (`Controller.UnPossess` (`self.GetController`))
  (`KismetSystemLibrary.Delay` 0.2)
  (bind _returnvalue (`|SpawnActorFromClass` "/Script/AIModule.AIController" (`self.GetTransform` self) "Undefined" "OverrideRootScale"))
  (`Controller.Possess` _returnvalue self)
  (`self.MoveUnderBall`))

(event `InputTouch`
  (params (Location :type "Vector Structure") (FingerIndex :type "ETouchIndex Enum")))

(event `SetCamera`
  (`KismetSystemLibrary.Delay` 0.2)
  (bind _outactors (`GameplayStatics.GetAllActorsOfClass` "/Game/Base/BP_OrthoCamera.BP_OrthoCamera_C"))
  (for _array_element _outactors
    (`PlayerController.SetViewTargetWithBlend` (cast `PlayerController` (`self.GetController`) :!pure true) _array_element 0.0 "VTBlend_Linear" 0.0 false)))

(event `self.ReceiveBeginPlay`
  (`KismetSystemLibrary.Delay` 1.0)
  (set `self.PaddleSpriteScale` (`SceneComponent.RelativeScale3D` (`self.PaperSprite`)))
  (if (`self.IsBot`)
    (`self.SetUpBot`)
    (else
      (`|SpawnActorFromClass` "/Game/Base/BP_PingPongBall.BP_PingPongBall_C" (`KismetMathLibrary.MakeTransform` (0.0 0.0 1000.0) (struct :`Pitch` 90.0)) "Undefined" "OverrideRootScale" null 800.0)
      (`self.SetCamera`)
      (set `PlayerController.bShowMouseCursor` true (cast `PlayerController` (`self.GetController`) :!pure true)))))

(event `InputAxis|PaddleMovement`
  (params (AxisValue :type "Float (single-precision)"))
  (`self.AddMovementInput` self (0.0 1.0 0.0) AxisValue false))

(event `self.ReceiveTick`
  (params (DeltaSeconds :type "Float (single-precision)"))
  (bind (_worldlocation _worlddirection) (`PlayerController.DeprojectMousePositionToWorld` (cast `PlayerController` (`self.GetController`) :!pure true)))
  (bind _returnvalue (`KismetMathLibrary.MakeVector` 0.0 (.y (+ _worldlocation (* (* _worlddirection (/ (.x _worldlocation) (.x _worlddirection))) -1.0))) (.z (+ _worldlocation (* (* _worlddirection (/ (.x _worldlocation) (.x _worlddirection))) -1.0)))))
  (if (`self.IsBot`)
    (`self.K2_SetActorLocation` (`KismetMathLibrary.MakeVector` (.x (`self.K2_GetActorLocation`)) (`KismetMathLibrary.FClamp` (.y (`self.K2_GetActorLocation`)) (`self.Clamp_Min`) (`self.Clamp_Max`)) (.z (`self.K2_GetActorLocation`))))
    (else
      (`SceneComponent.K2_SetWorldLocation` (`self.Cube`) _returnvalue false false)
      (`self.K2_SetActorRotation` (`KismetMathLibrary.FindLookAtRotation` (`KismetMathLibrary.MakeVector` 0.0 (.y (`self.K2_GetActorLocation`)) (.z (`self.K2_GetActorLocation`))) _returnvalue)))))

(event `Key|LeftMouseButton`
  (params (Key :type "Key Structure" :default "AnyKey"))
  (bind _powered (`self.Powered`))
  (bind _paddle (`self.Paddle`))
  (:`Pressed`
    (if (not (or _powered (`self.Weakened`))) :!label _label
      (set `self.Powered` true)
      (bind (_direction _meshscale _colliderscale _paddlespritescale) (`Timeline|StretchPower` :!via `PlayFromStart` :!label _label_2)
        (:`Update`
          (`SceneComponent.SetRelativeScale3D` _paddle (`KismetMathLibrary.MakeVector` (.x (`SceneComponent.RelativeScale3D` _paddle)) _meshscale (.z (`SceneComponent.RelativeScale3D` _paddle))))
          (`BoxComponent.SetBoxExtent` (`self.Box`) (`KismetMathLibrary.MakeVector` 50.0 _colliderscale 50.0) false)
          (`SceneComponent.SetRelativeScale3D` (`self.PaperSprite`) (`KismetMathLibrary.MakeVector` (* _paddlespritescale (.x (`self.PaddleSpriteScale`))) (.y (`self.PaddleSpriteScale`)) (.z (`self.PaddleSpriteScale`))))
          (bind _returnvalue (+ (- 200.0 _colliderscale) 310.0))
          (set `self.Clamp_Min` (* _returnvalue -1.0))
          (set `self.Clamp_Max` _returnvalue)))))
  (:`Released`
    (if _powered :!label _label_3
      (set `self.Powered` false)
      (goto _label_2 :!via `ReverseFromEnd`))))

(event `BotLeftClick`
  (bind _isa (`/Engine/EditorBlueprintResources/StandardMacros.FlipFlop`)
    (:`A`
      (goto _label))
    (:`B`
      (goto _label_3))))

(event `BotResetPaddle`
  (bind _paddle (`self.Paddle`))
  (`|ExecutionSequence`
    (:`then_0`
      (if (not (stale `BotLeftClick` _isa))
        (goto _label_3)))
    (:`then_1`
      (if (not (stale `Bot_RightClick` _isa))
        (if (`self.Weakened`) :!label _label_4
          (set `self.Weakened` false)
          (bind (_direction _meshscale _colliderscale _paddlespritescale) (`Timeline|StretchWeak` :!via `ReverseFromEnd` :!label _label_5)
            (:`Update`
              (`SceneComponent.SetRelativeScale3D` _paddle (`KismetMathLibrary.MakeVector` (.x (`SceneComponent.RelativeScale3D` _paddle)) _meshscale (.z (`SceneComponent.RelativeScale3D` _paddle))))
              (`BoxComponent.SetBoxExtent` (`self.Box`) (`KismetMathLibrary.MakeVector` 50.0 _colliderscale 50.0) false)
              (`SceneComponent.SetRelativeScale3D` (`self.PaperSprite`) (`KismetMathLibrary.MakeVector` (* _paddlespritescale (.x (`self.PaddleSpriteScale`))) (.y (`self.PaddleSpriteScale`)) (.z (`self.PaddleSpriteScale`))))
              (bind _returnvalue (- 310.0 (- _colliderscale 200.0)))
              (set `self.Clamp_Min` (* _returnvalue -1.0))
              (set `self.Clamp_Max` _returnvalue))))))))

(event `Key|RightMouseButton`
  (params (Key :type "Key Structure" :default "AnyKey"))
  (:`Pressed`
    (if (not (or (`self.Powered`) (`self.Weakened`))) :!label _label_6
      (set `self.Weakened` true)
      (goto _label_5 :!via `PlayFromStart`)))
  (:`Released`
    (goto _label_4)))

(event `Bot_RightClick`
  (bind _isa (`/Engine/EditorBlueprintResources/StandardMacros.FlipFlop`)
    (:`A`
      (goto _label_6))
    (:`B`
      (goto _label_4))))

(event `self.Box.OnComponentHit`
  (params (HitComponent :type "PrimitiveComponent Object Reference") (OtherActor :type "Actor Object Reference") (OtherComp :type "PrimitiveComponent Object Reference") (NormalImpulse :type "Vector Structure") (Hit :type "HitResult Structure (by ref)"))
  (cast `/Game/Base/BP_PingPongBall` OtherActor)
  (if (`self.IsBot`)
    (switch `int` (`KismetMathLibrary.RandomInteger` 3)
      (:`0`
        (`self.BotLeftClick`))
      (:`1`
        (`self.Bot_RightClick`)))))

(fn `UserConstructionScript`)