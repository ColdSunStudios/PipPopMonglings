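; BP_Brick_01 is a breakable brick that loses a hit each time a BP_PingPongBall strikes its Cube.
; Remaining hits drive damage feedback: the Cube material changes, the stone mesh swaps to a damaged version on the last hit, and the actor is destroyed at zero.
; Overlapping BP_Borders teleports the brick to a fixed Y on the opposite side, wrapping it across the play area.
; Each non-final hit also prints the remaining count.
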(event `self.Cube.OnComponentHit`
  (params (HitComponent :type "PrimitiveComponent Object Reference") (OtherActor :type "Actor Object Reference") (OtherComp :type "PrimitiveComponent Object Reference") (NormalImpulse :type "Vector Structure") (Hit :type "HitResult Structure (by ref)"))
  (bind _cube (`self.Cube`))
  (cast `/Game/Base/BP_PingPongBall` OtherActor)
  (bind _output_get (set `self.HitsRemaining` (- (`self.HitsRemaining`) 1)))
  (if (== _output_get 0)
    (`self.K2_DestroyActor`)
    (else
      (`KismetSystemLibrary.PrintString` (`KismetStringLibrary.Conv_IntToString` _output_get))
      (switch `int` (`self.HitsRemaining`)
        (:`1`
          (`PrimitiveComponent.SetMaterial` _cube 0 "/Game/Environment/Materials/M_Brick_Low_01.M_Brick_Low_01")
          (`SceneComponent.SetVisibility` (`self.Stone_01`) false false)
          (`SceneComponent.SetVisibility` (`self.Stone_Damaged_01`) true false))
        (:`2`
          (`PrimitiveComponent.SetMaterial` _cube 0 "/Game/Environment/Materials/M_Brick_Mid_01.M_Brick_Mid_01"))))))

(event `self.Cube.OnComponentBeginOverlap`
  (params (OverlappedComponent :type "PrimitiveComponent Object Reference") (OtherActor :type "Actor Object Reference") (OtherComp :type "PrimitiveComponent Object Reference") (OtherBodyIndex :type Integer) (bFromSweep :type Boolean) (SweepResult :type "HitResult Structure (by ref)"))
  (bind _x (.x (`self.K2_GetActorLocation`)))
  (bind _z (.z (`self.K2_GetActorLocation`)))
  (cast `/Game/Base/BP_Borders` OtherActor)
  (if (> (.y (`self.K2_GetActorLocation`)) 0.0)
    (`self.K2_SetActorLocation` (`KismetMathLibrary.MakeVector` _x -450.0 _z))
    (else
      (`self.K2_SetActorLocation` (`KismetMathLibrary.MakeVector` _x 450.0 _z)))))

(fn `UserConstructionScript`)