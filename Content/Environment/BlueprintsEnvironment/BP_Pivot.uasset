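; BP_Pivot is a sprite-based pivot obstacle that flips between two tilted positions when struck by a BP_PingPongBall.
; Each of two box components snaps the actor's pitch to an opposite fixed angle on hit, keeping roll and yaw.
; The shared Flip event prints a debug message and briefly disables actor collision after rotating.
; The construction script rotates and offsets the pivot sprite when Mirrored is set; an older FlipFlop toggle remains unconnected.
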(event `self.SPR_Pivot.OnComponentBeginOverlap`
  (params (OverlappedComponent :type "PrimitiveComponent Object Reference") (OtherActor :type "Actor Object Reference") (OtherComp :type "PrimitiveComponent Object Reference") (OtherBodyIndex :type Integer) (bFromSweep :type Boolean) (SweepResult :type "HitResult Structure (by ref)")))

(event `self.SPR_Pivot.OnComponentHit`
  (params (HitComponent :type "PrimitiveComponent Object Reference") (OtherActor :type "Actor Object Reference") (OtherComp :type "PrimitiveComponent Object Reference") (NormalImpulse :type "Vector Structure") (Hit :type "HitResult Structure (by ref)")))

(event `Flip`
  (params (TargetRotation :type "Rotator Structure"))
  (`self.K2_SetActorRotation` TargetRotation)
  (`KismetSystemLibrary.PrintString` "Flip!")
  (`self.SetActorEnableCollision` false)
  (`KismetSystemLibrary.Delay` 0.3)
  (`self.SetActorEnableCollision` true))

(event `self.Box.OnComponentHit`
  (params (HitComponent :type "PrimitiveComponent Object Reference") (OtherActor :type "Actor Object Reference") (OtherComp :type "PrimitiveComponent Object Reference") (NormalImpulse :type "Vector Structure") (Hit :type "HitResult Structure (by ref)"))
  (cast `/Game/Base/BP_PingPongBall` OtherActor)
  (`self.Flip` (`KismetMathLibrary.MakeRotator` (.roll (`self.K2_GetActorRotation`)) -45.0 (.yaw (`self.K2_GetActorRotation`)))))

(event `self.Box1.OnComponentHit`
  (params (HitComponent :type "PrimitiveComponent Object Reference") (OtherActor :type "Actor Object Reference") (OtherComp :type "PrimitiveComponent Object Reference") (NormalImpulse :type "Vector Structure") (Hit :type "HitResult Structure (by ref)"))
  (cast `/Game/Base/BP_PingPongBall` OtherActor)
  (`self.Flip` (`KismetMathLibrary.MakeRotator` (.roll (`self.K2_GetActorRotation`)) 45.0 (.yaw (`self.K2_GetActorRotation`)))))

(fn `UserConstructionScript`
  (if (`self.Mirrored`)
    (`SceneComponent.K2_SetRelativeRotation` (`self.SPR_Pivot`) (struct :`Pitch` 180.0) false false)
    (`SceneComponent.K2_SetRelativeLocation` (`self.SPR_Pivot`) (-470.0 0.0 30.0) false false)))